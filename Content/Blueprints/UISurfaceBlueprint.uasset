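; UISurfaceBlueprint is an input front end for a UI surface, translating mouse and gamepad input into UI events.
; Click press and release, scroll up and down, and back each pair a mouse input with a gamepad equivalent, feeding one shared handler call.
; BeginPlay calls InitializeView; the handler logic is defined outside these graphs, and the construction script is empty.
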(event EventBeginPlay
  (Class|UISurfaceActor|InitializeView))

(event Input|GamepadEvents|GamepadFaceButtonBottom
  (:Pressed
    (Class|UISurfaceActor|HandleMouseDownEvent))
  (:Released
    (Class|UISurfaceActor|HandleMouseUpEvent)))

(event Input|MouseEvents|LeftMouseButton
  (:Pressed
    (Class|UISurfaceActor|HandleMouseDownEvent))
  (:Released
    (Class|UISurfaceActor|HandleMouseUpEvent)))

(event Input|MouseEvents|RightMouseButton
  (:Pressed
    (Class|UISurfaceActor|HandleBackEvent)))

(event Input|MouseEvents|MouseWheelDown
  (:Pressed
    (Class|UISurfaceActor|HandleScrollDownEvent)))

(event Input|GamepadEvents|GamepadDPadDown
  (:Pressed
    (Class|UISurfaceActor|HandleScrollDownEvent)))

(event Input|MouseEvents|MouseWheelUp
  (:Pressed
    (Class|UISurfaceActor|HandleScrollUpEvent)))

(event Input|GamepadEvents|GamepadDPadUp
  (:Pressed
    (Class|UISurfaceActor|HandleScrollUpEvent)))

(event Input|GamepadEvents|GamepadFaceButtonRight
  (:Pressed
    (Class|UISurfaceActor|HandleBackEvent)))

(fn ConstructionScript)